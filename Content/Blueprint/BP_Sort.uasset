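; BP_Sort is an actor that builds a row of randomly valued BP_Item bars, apparently for a sorting visualisation, though it contains no sorting logic.
; The construction script calls Init, which derives bar width and gap from Length and Amount, then rebuilds the Items array from child actor components.
; Each bar receives its width and random value through SetSize.
; ClacLocation supplies positions, but its centred Y-axis spacing formula appears unconnected.
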(fn ConstructionScript
  (CallFunction|Init))

(fn Init
  ;[1 1 1] Set Space 元素间隙
  (Variables|Default|SetSpace (/ (/ (Variables|Default|GetLength) 2.0) (Math|Conversions|ToFloat(Integer) (Variables|Default|GetAmount))))
  ;[1 1 1] Set Width 元素宽
  (Variables|Default|SetWidth (/ (- (Variables|Default|GetLength) (* (- (Variables|Default|GetAmount) 1) (Variables|Default|GetSpace))) (Math|Conversions|ToFloat(Integer) (Variables|Default|GetAmount))))
  ;[1 1 1] 每次构造清空元素数组Items
  (Utilities|Array|Clear (Variables|Default|GetItems))
  ;[1 1 1] 增加元素
  (for _index (range 0 (- (Variables|Default|GetAmount) 1))
    (bind _returnvalue (AddComponent|AddChildActorComponent false (Math|Transform|MakeTransform (Utilities|ClacLocation _index))))
    (bind _asbp_item (Utilities|Casting|CastToBP_Item (Variables|/Script/Engine.ChildActorComponent|GetChildActor _returnvalue)))
    (Default|SetSize _asbp_item (Variables|Default|GetWidth) (+ (Math|Random|RandomInteger 99) 1))
    (Utilities|Array|Add (Variables|Default|GetItems) _asbp_item)))