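; Selection sort visualizer Blueprint that animates the algorithm on an array of colored cube items, extending a parent sort class.
; Each DoSort call advances one step using persistent I, J and MinIndex instead of loops, clearing the timer handle when finished.
; Colors mark the compared item, current minimum and sorted items, with delays pacing the display.
; After each pass, Move animates the two cubes trading places before their array entries swap.
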(event EventBeginPlay
  (|CallParentFunction) ; This node is disabled and will not be called.\nDrag off pins to build functionality.
)

(event EventDoSort
  (bind _items (Variables|Default|GetItems))
  (bind _items_2 (Variables|Default|GetItems))
  ;[1 1 1] I<Length-1
  (if (< (Variables|Default|GetI) (- (Utilities|Array|Length (Variables|Default|GetItems)) 1))
    ;[0.2235 0 0] 将MinIndex元素设置为黄色
    (Default|SetColor (Utilities|Array|Get(acopy) (Variables|Default|GetItems) (Variables|Default|GetMinIndex)) "(R=0.223529,G=0.183566,B=0.001988,A=1.000000)")
    ;[1 1 1] J<Length
    (if (< (Variables|Default|GetJ) (Utilities|Array|Length (Variables|Default|GetItems)))
      ;[1 1 1] Set Info
      (Math|Integer|IncrementInt (Variables|Default|GetStepCount)
        (:%20%20
          (Variables|Default|SetInfo (Utilities|Text|ToText(String) (Utilities|String|Append "I:" (Utilities|String|ToString(Integer) (Variables|Default|GetI)) " " "J:" (Utilities|String|ToString(Integer) (Variables|Default|GetJ)))))
          ;[0.2235 0.1836 0.001988] 将J元素设置为红色
          (Default|SetColor (Utilities|Array|Get(acopy) (Variables|Default|GetItems) (Variables|Default|GetJ)) "(R=0.223529,G=0.000000,B=0.000000,A=1.000000)")
          ;[0.2235 0 0] 延迟SortTime
          (Utilities|FlowControl|Delay (Variables|Default|GetSortTime))
          ;[0.2235 0 0] 如果第J个元素值小于第MinIndex个元素值，将这个已经不是最小的MinIndex元素的颜色改为蓝色，将J元素改为黄色。MinIndex=J
          (if (< (Variables|/Game/Blueprint/BP_Item.BP_Item_C|GetValue (Utilities|Array|Get(acopy) _items (Variables|Default|GetJ))) (Variables|/Game/Blueprint/BP_Item.BP_Item_C|GetValue (Utilities|Array|Get(acopy) _items (Variables|Default|GetMinIndex))))
            (Default|SetColor (Utilities|Array|Get(acopy) _items_2 (Variables|Default|GetMinIndex)) "(R=0.000000,G=0.101961,B=0.180392,A=1.000000)")
            (Default|SetColor (Utilities|Array|Get(acopy) _items_2 (Variables|Default|GetJ)) "(R=0.223529,G=0.183566,B=0.001988,A=1.000000)")
            (Variables|Default|SetMinIndex (Variables|Default|GetJ))
            (else
              ;[0 0.102 0.1804] 如果还是MinIndex元素小，将J元素改为蓝色
              (Default|SetColor (Utilities|Array|Get(acopy) (Variables|Default|GetItems) (Variables|Default|GetJ)) "(R=0.000000,G=0.101961,B=0.180392,A=1.000000)")))
          (Math|Integer|IncrementInt (Variables|Default|GetJ))))
      (else
        (if (!= (Variables|Default|GetMinIndex) (Variables|Default|GetI))
          ;[0.2235 0 0] 将I元素元素设置为红色
          (Default|SetColor (Utilities|Array|Get(acopy) (Variables|Default|GetItems) (Variables|Default|GetI)) "(R=0.223529,G=0.000000,B=0.000000,A=1.000000)")
          ;[0.2235 0 0] 交换I元素和MinIndex元素的立方体位置
          (CallFunction|Move (Variables|Default|GetI) (Variables|Default|GetMinIndex))
          (CallFunction|Move (Variables|Default|GetMinIndex) (Variables|Default|GetI))
          ;[0.2235 0 0] 延迟SortTime
          (Utilities|FlowControl|Delay (Variables|Default|GetSortTime))
          ;[0 0.102 0.1804] 将I元素设置为蓝色
          (Default|SetColor (Utilities|Array|Get(acopy) (Variables|Default|GetItems) (Variables|Default|GetI)) "(R=0.000000,G=0.101961,B=0.180392,A=1.000000)")
          ;[0 0.102 0.1804] 如果MinIndex!=I，将第MinIndex个元素和第I个元素交换位置
          (Variables|Default|SetBP_ItemTemp (Utilities|Array|Get(acopy) (Variables|Default|GetItems) (Variables|Default|GetI)))
          (Utilities|Array|SetArrayElem (Variables|Default|GetItems) (Variables|Default|GetI) (Utilities|Array|Get(acopy) (Variables|Default|GetItems) (Variables|Default|GetMinIndex)))
          (Utilities|Array|SetArrayElem (Variables|Default|GetItems) (Variables|Default|GetMinIndex) (Variables|Default|GetBP_ItemTemp)))
        ;[0.001582 0.1594 0.02441] 将I元素设置为绿色
        (Default|SetColor (Utilities|Array|Get(acopy) (Variables|Default|GetItems) (Variables|Default|GetI)) "(R=0.001582,G=0.159375,B=0.024405,A=1.000000)")
        ;[0.001582 0.1594 0.02441] 执行完一轮J。I++，MinIndex=I， J=I+1
        (bind _result (Math|Integer|IncrementInt (Variables|Default|GetI))
          (:%20%20
            (bind _output_get (Variables|Default|SetMinIndex _result))
            (Variables|Default|SetJ (+ _output_get 1))))))
    (else
      ;[0.001582 0.1594 0.02441] 将I元素设置为绿色
      (Default|SetColor (Utilities|Array|Get(acopy) (Variables|Default|GetItems) (Variables|Default|GetI)) "(R=0.001582,G=0.159375,B=0.024405,A=1.000000)")
      ;[0.001582 0.1594 0.02441] Clear Timer
      (Utilities|Time|ClearandInvalidateTimerbyHandle (Variables|Default|GetTimerHandle)))))

(fn ConstructionScript
  (|CallParentFunction))

(fn Move
  (params (InLastIndex :type Integer) (InTargetIndex :type Integer))
  (bind _outlocation (CallFunction|GetItemLocation InLastIndex))
  (bind _outlocation_2 (CallFunction|GetItemLocation InTargetIndex))
  (Default|Move (Utilities|Array|Get(acopy) (Variables|Default|GetItems) InLastIndex) _outlocation _outlocation_2 (* (Class|KismetMathLibrary|SignOfInteger (- InTargetIndex InLastIndex)) (Variables|Default|GetWidth))))

(fn Init
  (params (InAmount :type Integer) (InLength :type Float%20%28single-precision%29) (InSortTime :type Float%20%28single-precision%29))
  (|CallParentFunction InAmount InLength InSortTime)
  (bind _output_get (Variables|Default|SetI 0))
  (Variables|Default|SetMinIndex _output_get)
  (Variables|Default|SetJ 1)
  (Variables|Default|SetBP_ItemTemp 0))