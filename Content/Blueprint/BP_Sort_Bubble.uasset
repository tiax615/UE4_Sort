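; Bubble sort visualizer, a child Blueprint that animates item actors being sorted by value.
; Each DoSort call makes one comparison, tracking I and J across calls, counting steps and updating debug text.
; Compared pairs turn red, animate swaps through Move, and update the array after a SortTime delay.
; Each pass's final item turns green, and the timer is cleared once sorting ends.
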(event EventBeginPlay
  (|CallParentFunction))

(event EventDoSort
  (bind _items (Variables|Default|GetItems))
  (bind _items_2 (Variables|Default|GetItems))
  (bind _items_3 (Variables|Default|GetItems))
  ;[1 1 1] I<Items.Length
  (if (< (Variables|Default|GetI) (Utilities|Array|Length (Variables|Default|GetItems)))
    ;[1 1 1] J<Items.Length-1-I
    (if (< (Variables|Default|GetJ) (- (- (Utilities|Array|Length (Variables|Default|GetItems)) 1) (Variables|Default|GetI)))
      ;[1 1 1] Set Info
      (Variables|Default|SetInfo (Utilities|Text|ToText(String) (Utilities|String|Append "I:" (Utilities|String|ToString(Integer) (Variables|Default|GetI)) " " "J:" (Utilities|String|ToString(Integer) (Variables|Default|GetJ)))))
      ;[1 1 1] 记录进行比较的次数
      (Math|Integer|IncrementInt (Variables|Default|GetStepCount)
        (:%20%20
          ;[1 0 0] 将正要进行比较的两个元素，设置为红色
          (Default|SetColor (Utilities|Array|Get(acopy) _items_3 (Variables|Default|GetJ)) "(R=0.223529,G=0.000000,B=0.000000,A=1.000000)")
          (Default|SetColor (Utilities|Array|Get(acopy) _items_3 (+ (Variables|Default|GetJ) 1)) "(R=0.223529,G=0.000000,B=0.000000,A=1.000000)")
          ;[1 0 0] J元素值比J+1元素值大，交换两元素位置。等待SortTime后，交换两个元素在数组Items中的位置。
          (if (> (Variables|/Game/Blueprint/BP_Item.BP_Item_C|GetValue (Utilities|Array|Get(acopy) _items (Variables|Default|GetJ))) (Variables|/Game/Blueprint/BP_Item.BP_Item_C|GetValue (Utilities|Array|Get(acopy) _items (+ (Variables|Default|GetJ) 1))))
            (CallFunction|Move (Variables|Default|GetJ) (+ (Variables|Default|GetJ) 1))
            (CallFunction|Move (+ (Variables|Default|GetJ) 1) (Variables|Default|GetJ))
            (Utilities|FlowControl|Delay (Variables|Default|GetSortTime))
            (Variables|Default|SetBP_ItemTemp (Utilities|Array|Get(acopy) (Variables|Default|GetItems) (+ (Variables|Default|GetJ) 1)))
            (Utilities|Array|SetArrayElem (Variables|Default|GetItems) (+ (Variables|Default|GetJ) 1) (Utilities|Array|Get(acopy) (Variables|Default|GetItems) (Variables|Default|GetJ)) true)
            (Utilities|Array|SetArrayElem (Variables|Default|GetItems) (Variables|Default|GetJ) (Variables|Default|GetBP_ItemTemp) true)
            (else
              ;[1 0 0] J元素值没有J+1元素值大，等待SortTime
              (Utilities|FlowControl|Delay (Variables|Default|GetSortTime))))
          ;[0 0 1] 执行完一次元素比较，还原颜色。J++
          (Default|SetColor (Utilities|Array|Get(acopy) _items_2 (Variables|Default|GetJ)) "(R=0.000000,G=0.101961,B=0.180392,A=1.000000)")
          (Default|SetColor (Utilities|Array|Get(acopy) _items_2 (+ (Variables|Default|GetJ) 1)) "(R=0.000000,G=0.101961,B=0.180392,A=1.000000)")
          (Math|Integer|IncrementInt (Variables|Default|GetJ))))
      (else
        ;[0 1 0] 每次J循环结束，修改第J个元素的颜色，I++，J=0
        (Math|Integer|IncrementInt (Variables|Default|GetI)
          (:%20%20
            (Default|SetColor (Utilities|Array|Get(acopy) (Variables|Default|GetItems) (Variables|Default|GetJ)) "(R=0.001582,G=0.159375,B=0.024405,A=1.000000)")
            (Variables|Default|SetJ 0)))))
    (else
      ;[0 1 0] Clear Timer
      (Utilities|Time|ClearandInvalidateTimerbyHandle (Variables|Default|GetTimerHandle)))))

(fn ConstructionScript
  (|CallParentFunction))

(fn Move
  (params (InLastIndex :type Integer) (InTargetIndex :type Integer))
  (Default|Move (Utilities|Array|Get(acopy) (Variables|Default|GetItems) InLastIndex) (Utilities|ClacLocation InLastIndex) (Utilities|ClacLocation InTargetIndex) (* (Class|KismetMathLibrary|SignOfInteger (- InTargetIndex InLastIndex)) (Variables|Default|GetWidth))))

(fn Init
  (params (InAmount :type Integer) (InLength :type Float%20%28single-precision%29) (InSortTime :type Float%20%28single-precision%29))
  (|CallParentFunction InAmount InLength InSortTime)
  (Variables|Default|SetI 0)
  (Variables|Default|SetJ 0)
  (Variables|Default|SetBP_ItemTemp 0))