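; Merge sort visualizer, a child Blueprint that animates bottom-up merge sort on bar items with Value, color and movement.
; Each DoSort call advances an ActionIndex state machine: color both runs red and yellow, compare, drain leftovers, write back in green.
; Merged items slide out along X into TempItems, then return to Items.
; Gap doubles each pass until it covers the array, then the timer is cleared.
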(event EventBeginPlay
  (|CallParentFunction))

(event EventDoSort
  ;[1 1 1] Set Info
  (Variables|Default|SetInfo (Utilities|Text|ToText(String) (Utilities|String|Append "Gap:" (Utilities|String|ToString(Integer) (Variables|Default|GetGap)) " " "Next:" (Utilities|String|ToString(Integer) (Variables|Default|GetNext)))))
  ;[1 1 1] If Gap<Items.Length ?
  (if (< (Variables|Default|GetGap) (Variables|Default|GetItemsLength))
    ;[1 1 1] If LeftMin<ItemsLength-Gap ?
    (if (< (Variables|Default|GetNext) (Variables|Default|GetItemsLength))
      ;[1 1 1] ActionIndex:
      ; 0: Init
      ; 1: 比较左边和右边，将小的增加到TempItems
      ; 2: 处理左边或右边没加入TempItems的部分
      (switch int (Variables|Default|GetActionIndex)
        (:0
          ;[1 1 1] 0: 每次Gap循环的初始化
          (bind _output_get (Variables|Default|SetLeftMax (+ (Variables|Default|GetLeftMin) (Variables|Default|GetGap))))
          (bind _output_get_2 (Variables|Default|SetRightMin _output_get))
          (Variables|Default|SetRightMax (+ _output_get_2 (Variables|Default|GetGap)))
          ;;[1 1 1] 右边下标的最大值只能为ItemsLength
          (if (> (Variables|Default|GetRightMax) (Variables|Default|GetItemsLength))
            (Variables|Default|SetRightMax (Variables|Default|GetItemsLength)))
          ;[0.2235 0.1836 0.001988] 将Left元素标红，Right元素标黄。完成后ActionIndex=1
          (for _index (range (Variables|Default|GetLeftMin) (- (Variables|Default|GetLeftMax) 1))
            (if (< _index (Variables|Default|GetItemsLength))
              (Default|SetColor (Utilities|Array|Get(acopy) (Variables|Default|GetItems) _index) "(R=0.223529,G=0.000000,B=0.000000,A=1.000000)")))
          (for _index_2 (range (Variables|Default|GetRightMin) (- (Variables|Default|GetRightMax) 1))
            (Default|SetColor (Utilities|Array|Get(acopy) (Variables|Default|GetItems) _index_2) "(R=0.223529,G=0.183566,B=0.001988,A=1.000000)"))
          (Utilities|FlowControl|Delay (Variables|Default|GetSortTime))
          (Variables|Default|SetActionIndex 1))
        (:1
          ;[1 1 1] If 左边的数据没到分隔线 && 右边的数据没到分隔线
          (if (and (< (Variables|Default|GetLeftMin) (Variables|Default|GetLeftMax)) (< (Variables|Default|GetRightMin) (Variables|Default|GetRightMax)))
            (Math|Integer|IncrementInt (Variables|Default|GetStepCount)
              (:%20%20
                ;[0.2235 0 0] If 左边第LeftMin值<右边第RightMin值 ?
                (if (< (Variables|/Game/Blueprint/BP_Item.BP_Item_C|GetValue (Utilities|Array|Get(acopy) (Variables|Default|GetItems) (Variables|Default|GetLeftMin))) (Variables|/Game/Blueprint/BP_Item.BP_Item_C|GetValue (Utilities|Array|Get(acopy) (Variables|Default|GetItems) (Variables|Default|GetRightMin))))
                  ;[0.2235 0 0] 可视化：左边第LeftMin元素移出到Next位置
                  (CallFunction|Move (Variables|Default|GetLeftMin) (Variables|Default|GetNext) true :!label _label)
                  (Utilities|FlowControl|Delay (Variables|Default|GetSortTime))
                  ;[0.2235 0 0] LeftMin元素Append到TempItems，LeftMin++,Next++
                  (Utilities|Array|Add (Variables|Default|GetTempItems) (Utilities|Array|Get(acopy) (Variables|Default|GetItems) (Variables|Default|GetLeftMin)))
                  (Math|Integer|IncrementInt (Variables|Default|GetLeftMin)
                    (:%20%20
                      (Math|Integer|IncrementInt (Variables|Default|GetNext))))
                  (else
                    ;[0.2235 0.1836 0.001988] 可视化：右边第RightMin元素移出到Next位置
                    (CallFunction|Move (Variables|Default|GetRightMin) (Variables|Default|GetNext) true :!label _label_2)
                    (Utilities|FlowControl|Delay (Variables|Default|GetSortTime))
                    ;[0.2235 0.1836 0.001988] RightMin元素Append到TempItems，RightMin++,Next++
                    (Utilities|Array|Add (Variables|Default|GetTempItems) (Utilities|Array|Get(acopy) (Variables|Default|GetItems) (Variables|Default|GetRightMin)))
                    (Math|Integer|IncrementInt (Variables|Default|GetRightMin)
                      (:%20%20
                        (Math|Integer|IncrementInt (Variables|Default|GetNext))))))))
            (else
              ;[1 1 1] 左边到了分隔线 || 右边到了分隔线，ActionIndex=2
              (Variables|Default|SetActionIndex 2))))
        (:2
          ;[0.2235 0 0] 左边没排完
          (if (< (Variables|Default|GetLeftMin) (Variables|Default|GetLeftMax))
            (goto _label)
            (else
              ;[0.2235 0.1836 0.001988] 右边没排完
              (if (< (Variables|Default|GetRightMin) (Variables|Default|GetRightMax))
                (goto _label_2)
                (else
                  ;[0.001582 0.1594 0.02441] 排完了，ActionIndex=3
                  (Variables|Default|SetActionIndex 3))))))
        (:3
          ;[0.001582 0.1594 0.02441] 完成这轮排序，将TempItems中(LeftMin-Gap)到(Next-1)元素标绿，返回到Items，并移回柱状图
          (for _index_3 (range (- (Variables|Default|GetLeftMin) (Variables|Default|GetGap)) (- (Variables|Default|GetNext) 1))
            (Default|SetColor (Utilities|Array|Get(acopy) (Variables|Default|GetTempItems) _index_3) "(R=0.001582,G=0.159375,B=0.024405,A=1.000000)")
            (Utilities|Array|SetArrayElem (Variables|Default|GetItems) _index_3 (Utilities|Array|Get(acopy) (Variables|Default|GetTempItems) _index_3))
            (CallFunction|Move _index_3 _index_3 false))
          (Utilities|FlowControl|Delay (Variables|Default|GetSortTime))
          (Variables|Default|SetLeftMin (Variables|Default|GetRightMax))
          (Variables|Default|SetActionIndex 0)))
      (else
        ;[0.001582 0.1594 0.02441] 完成这轮排序，将TempItems中(LeftMin-Gap)到(Next-1)元素标绿，返回到Items，并移回柱状图
        (for _index_4 (range (- (Variables|Default|GetLeftMin) (Variables|Default|GetGap)) (- (Variables|Default|GetNext) 1))
          (Default|SetColor (Utilities|Array|Get(acopy) (Variables|Default|GetTempItems) _index_4) "(R=0.001582,G=0.159375,B=0.024405,A=1.000000)")
          (Utilities|Array|SetArrayElem (Variables|Default|GetItems) _index_4 (Utilities|Array|Get(acopy) (Variables|Default|GetTempItems) _index_4))
          (CallFunction|Move _index_4 _index_4 false))
        (Utilities|FlowControl|Delay (Variables|Default|GetSortTime))
        (Variables|Default|SetLeftMin (Variables|Default|GetRightMax))
        (Variables|Default|SetActionIndex 0)
        ;[0.001582 0.1594 0.02441] 开启下轮排序。Gap=*2,LeftMin=0
        (Variables|Default|SetLeftMin 0)
        (Variables|Default|SetGap (* (Variables|Default|GetGap) 2))
        (Variables|Default|SetNext 0)
        (Utilities|Array|Clear (Variables|Default|GetTempItems))))
    (else
      ;[0.001582 0.1594 0.02441] Finish
      (Utilities|Time|ClearandInvalidateTimerbyHandle (Variables|Default|GetTimerHandle))
      (Variables|Default|SetInfo "Finish"))))

(fn ConstructionScript
  (|CallParentFunction))

(fn Init
  (params (InAmount :type Integer) (InLength :type Float%20%28single-precision%29) (InSortTime :type Float%20%28single-precision%29))
  (|CallParentFunction InAmount InLength InSortTime)
  (Variables|Default|SetGap 1)
  (Variables|Default|SetNext 0)
  (Variables|Default|SetLeftMin 0)
  (Variables|Default|SetLeftMax 1)
  (Variables|Default|SetRightMin 1)
  (Variables|Default|SetRightMax 2)
  (Utilities|Array|Clear (Variables|Default|GetTempItems))
  (Variables|Default|SetActionIndex 0)
  (Variables|Default|SetItemsLength (Utilities|Array|Length (Variables|Default|GetItems))))

(fn Move
  (params (InLastIndex :type Integer) (InTargetIndex :type Integer) (IsOut :type Boolean))
  (bind _items (Variables|Default|GetItems))
  (bind _width (Variables|Default|GetWidth))
  (bind _returnvalue (* _width 2.0))
  (bind _output (Utilities|Array|Get(acopy) _items InLastIndex))
  (bind _returnvalue_2 (Math|Vector|MakeVector _returnvalue 0.0 0.0))
  (bind _returnvalue_3 (- "0, 0, 0" _returnvalue_2))
  (bind _outlocation (CallFunction|GetItemLocation InLastIndex))
  (bind _outlocation_2 (CallFunction|GetItemLocation InTargetIndex))
  (if IsOut
    (Default|Move _output _outlocation (+ _outlocation_2 _returnvalue_3) 0.0)
    (else
      (Default|Move _output (+ _outlocation _returnvalue_3) _outlocation_2 0.0))))