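; BP_Sort_Heap is an unfinished heap sort variant of a parent sorting Blueprint.
; Init passes amount, length and sort time to the parent, then clears the Temp element.
; DoSort is empty; unconnected fragments sketch a max-heap sift-down that stores the current item, picks the larger child and compares it with Temp, without any swap or loop.
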(event EventBeginPlay
  (|CallParentFunction) ; This node is disabled and will not be called.\nDrag off pins to build functionality.
)

(event EventDoSort)

(fn ConstructionScript
  (|CallParentFunction))

(fn Init
  (params (InAmount :type Integer) (InLength :type Float%20%28single-precision%29) (InSortTime :type Float%20%28single-precision%29))
  (|CallParentFunction InAmount InLength InSortTime)
  (Variables|Default|SetTemp 0))