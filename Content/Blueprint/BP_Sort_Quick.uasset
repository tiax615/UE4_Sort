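; Quick sort visualizer, a child sort Blueprint that animates Items being partitioned and reordered by Value.
; DoSort is a timer-driven, three-state machine (load range, partition step, finish partition) using the leftmost element as a Lomuto-style pivot.
; SortBuffer replaces recursion, queuing sub-range bounds first-in, first-out until empty.
; MoveX slides the active range out and back, MoveY animates swaps, and colors mark pivot, comparisons and sorted items.
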(event EventBeginPlay
  (|CallParentFunction) ; This node is disabled and will not be called.\nDrag off pins to build functionality.
)

(event EventDoSort
  (bind _sortbuffer (Variables|Default|GetSortBuffer))
  (bind _sortbuffer_2 (Variables|Default|GetSortBuffer))
  (bind _sortbuffer_3 (Variables|Default|GetSortBuffer))
  (bind _items (Variables|Default|GetItems))
  (switch int (Variables|Default|GetActionIndex)
    (:0
      ;[1 1 1] 将SortBuffer[0]给到Left，将SortBuffer[1]给到Right，并移出这两位。初始化Pivot,Index,I
      (bind _output_get (Variables|Default|SetLeft (Utilities|Array|Get(acopy) (Variables|Default|GetSortBuffer))))
      (bind _output_get_2 (Variables|Default|SetPivot _output_get))
      (bind _output_get_3 (Variables|Default|SetIndex (+ _output_get_2 1)))
      (Variables|Default|SetI _output_get_3)
      (Variables|Default|SetRight (Utilities|Array|Get(acopy) (Variables|Default|GetSortBuffer) 1))
      (Utilities|Array|RemoveIndex _sortbuffer_3)
      (Utilities|Array|RemoveIndex _sortbuffer_3)
      ;[0.2235 0 0] 可视化：基准元素标红
      (Default|SetColor (Utilities|Array|Get(acopy) (Variables|Default|GetItems) (Variables|Default|GetPivot)) "(R=0.223529,G=0.000000,B=0.000000,A=1.000000)")
      ;[1 1 1] 可视化：本次分区的所有柱子移出
      (for _index (range (Variables|Default|GetLeft) (Variables|Default|GetRight))
        (CallFunction|MoveX _index true))
      (Variables|Default|SetActionIndex 1))
    (:1
      ;[1 1 1] Set Info
      (Math|Integer|IncrementInt (Variables|Default|GetStepCount)
        (:%20%20
          (Variables|Default|SetInfo (Utilities|Text|ToText(String) (Utilities|String|Append "L:" (Utilities|String|ToString(Integer) (Variables|Default|GetLeft)) " " "R:" (Utilities|String|ToString(Integer) (Variables|Default|GetRight)) " " "I:" (Utilities|String|ToString(Integer) (Variables|Default|GetI)))))
          ;[1 1 1] 1: If I<=Right
          (if (<= (Variables|Default|GetI) (Variables|Default|GetRight))
            ;[1 1 1] If I值<Pivot值 ？
            (if (< (Variables|/Game/Blueprint/BP_Item.BP_Item_C|GetValue (Utilities|Array|Get(acopy) _items (Variables|Default|GetI))) (Variables|/Game/Blueprint/BP_Item.BP_Item_C|GetValue (Utilities|Array|Get(acopy) _items (Variables|Default|GetPivot))))
              ;[0.351 0.1169 0.1569] 可视化：I值<Pivot值，I元素标粉，交换I和Index位置。（小值放在Index左边）
              (Default|SetColor (Utilities|Array|Get(acopy) (Variables|Default|GetItems) (Variables|Default|GetI)) "(R=0.351042,G=0.116929,B=0.156950,A=1.000000)")
              (CallFunction|MoveY (Variables|Default|GetI) (Variables|Default|GetIndex))
              (CallFunction|MoveY (Variables|Default|GetIndex) (Variables|Default|GetI))
              (Utilities|FlowControl|Delay (Variables|Default|GetSortTime))
              ;[0.351 0.1169 0.1569] 交换I和Index索引，Index++,I++
              (Utilities|Array|Swap (Variables|Default|GetItems) (Variables|Default|GetI) (Variables|Default|GetIndex))
              (Math|Integer|IncrementInt (Variables|Default|GetIndex)
                (:%20%20
                  (Math|Integer|IncrementInt (Variables|Default|GetI))))
              (else
                ;[0.2235 0.1836 0.001988] 可视化：I元素标黄。（大值放在Index右边）
                (Default|SetColor (Utilities|Array|Get(acopy) (Variables|Default|GetItems) (Variables|Default|GetI)) "(R=0.223529,G=0.183566,B=0.001988,A=1.000000)")
                (Utilities|FlowControl|Delay (Variables|Default|GetSortTime))
                ;[0.2235 0.1836 0.001988] I++
                (Math|Integer|IncrementInt (Variables|Default|GetI))))
            (else
              ;[0.2235 0 0] 可视化：完成分区Partition，将Pivot元素和Index元素交换。（基准放在中间）
              (CallFunction|MoveY (Variables|Default|GetPivot) (- (Variables|Default|GetIndex) 1))
              (CallFunction|MoveY (- (Variables|Default|GetIndex) 1) (Variables|Default|GetPivot))
              (Utilities|FlowControl|Delay (Variables|Default|GetSortTime))
              ;[0.2235 0 0] 交换Pivot和Index索引
              (Utilities|Array|Swap (Variables|Default|GetItems) (Variables|Default|GetPivot) (- (Variables|Default|GetIndex) 1))
              (Variables|Default|SetActionIndex 2))))))
    (:2
      ;[0.07899 0.1728 0.1804] 可视化：将已本次分区元素标青
      (for _index_2 (range (Variables|Default|GetLeft) (Variables|Default|GetRight))
        (Default|SetColor (Utilities|Array|Get(acopy) (Variables|Default|GetItems) _index_2) "(R=0.078990,G=0.172848,B=0.180392,A=1.000000)"))
      ;[0.001582 0.1594 0.02441] 可视化：基准标绿，已排好序
      (Default|SetColor (Utilities|Array|Get(acopy) (Variables|Default|GetItems) (- (Variables|Default|GetIndex) 1)) "(R=0.001582,G=0.159375,B=0.024405,A=1.000000)")
      ;[1 1 1] 可视化：本次分区的所有柱子移入
      (for _index_3 (range (Variables|Default|GetLeft) (Variables|Default|GetRight))
        (CallFunction|MoveX _index_3 false))
      (Utilities|FlowControl|Delay (Variables|Default|GetSortTime))
      (Utilities|FlowControl|Sequence
        (:then_0
          ;[1 1 1] If Left<Pivot-1，左边还要分区，将左边的左Left右Pivot-1存入SortBuffer
          (if (< (Variables|Default|GetLeft) (- (Variables|Default|GetIndex) 2))
            (Utilities|Array|Add _sortbuffer_2 (Variables|Default|GetLeft))
            (Utilities|Array|Add _sortbuffer_2 (- (Variables|Default|GetIndex) 2))
            (else
              ;[0.001582 0.1594 0.02441] 左边排序OK，标绿
              (Default|SetColor (Utilities|Array|Get(acopy) (Variables|Default|GetItems) (Variables|Default|GetLeft)) "(R=0.001582,G=0.159375,B=0.024405,A=1.000000)"))))
        (:then_1
          ;[1 1 1] If Right>Pivot+1，右边还要分区，将右边的左Pivot+1右Right存入SortBuffer
          (if (> (Variables|Default|GetRight) (Variables|Default|GetIndex))
            (Utilities|Array|Add _sortbuffer (Variables|Default|GetIndex))
            (Utilities|Array|Add _sortbuffer (Variables|Default|GetRight))
            (else
              ;[0.001582 0.1594 0.02441] 右边排序OK，标绿
              (Default|SetColor (Utilities|Array|Get(acopy) (Variables|Default|GetItems) (Variables|Default|GetRight)) "(R=0.001582,G=0.159375,B=0.024405,A=1.000000)"))))
        (:then_2
          ;[1 1 1] If SortBuffer.Length>0，开始下轮分区；否则完成排序
          (if (> (Utilities|Array|Length (Variables|Default|GetSortBuffer)) 0)
            (Variables|Default|SetActionIndex 0)
            (else
              (Utilities|Time|ClearandInvalidateTimerbyHandle (Variables|Default|GetTimerHandle))
              (Variables|Default|SetInfo "Finish"))))))))

(fn ConstructionScript
  (|CallParentFunction))

(fn Init
  (params (InAmount :type Integer) (InLength :type Float%20%28single-precision%29) (InSortTime :type Float%20%28single-precision%29))
  (bind _sortbuffer (Variables|Default|GetSortBuffer))
  (|CallParentFunction InAmount InLength InSortTime)
  (Utilities|Array|Clear (Variables|Default|GetSortBuffer))
  (Utilities|Array|Add _sortbuffer 0)
  (Utilities|Array|Add _sortbuffer (- (Utilities|Array|Length (Variables|Default|GetItems)) 1))
  (Variables|Default|SetActionIndex 0))

(fn MoveX
  (params (InLastIndex :type Integer) (IsOut :type Boolean))
  (bind _items (Variables|Default|GetItems))
  (bind _output (Utilities|Array|Get(acopy) _items InLastIndex))
  (bind _outlocation (CallFunction|GetItemLocation InLastIndex))
  (if IsOut
    (Default|Move _output _outlocation (+ _outlocation (Math|Vector|MakeVector -8e+01 0.0 0.0)) 0.0)
    (else
      (Default|Move _output (+ _outlocation (Math|Vector|MakeVector -8e+01 0.0 0.0)) _outlocation 0.0))))

(fn MoveY
  (params (InLastIndex :type Integer) (InTargetIndex :type Integer))
  (bind _returnvalue (Math|Vector|MakeVector -8e+01 0.0 0.0))
  (bind _outlocation (CallFunction|GetItemLocation InLastIndex))
  (bind _outlocation_2 (CallFunction|GetItemLocation InTargetIndex))
  (Default|Move (Utilities|Array|Get(acopy) (Variables|Default|GetItems) InLastIndex) (+ _outlocation _returnvalue) (+ _outlocation_2 _returnvalue) (* (Class|KismetMathLibrary|SignOfInteger (- InTargetIndex InLastIndex)) (Variables|Default|GetWidth))))