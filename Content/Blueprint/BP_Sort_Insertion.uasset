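; BP_Sort_Insertion is a step-based insertion sort visualizer built on a parent that supplies BeginPlay and construction.
; DoSort tints item J red, updates the step count and I/J text, and compares it with its left neighbor, but that comparison leads to no action.
; When J reaches zero, I advances and J resets.
; MoveX and MoveY animate items between slots, MoveY offset along X, though neither is called here.
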(event EventBeginPlay
  (|CallParentFunction) ; This node is disabled and will not be called.\nDrag off pins to build functionality.
)

(event EventDoSort
  (bind _items (Variables|Default|GetItems))
  ;[1 1 1] I<Length-1
  (if (< (Variables|Default|GetI) (- (Utilities|Array|Length (Variables|Default|GetItems)) 1))
    ;[1 1 1] J>0
    (if (> (Variables|Default|GetJ) 0)
      ;[1 1 1] J元素标红
      (Default|SetColor (Utilities|Array|Get(acopy) (Variables|Default|GetItems) (Variables|Default|GetJ)) "(R=0.223529,G=0.000000,B=0.000000,A=1.000000)")
      ;[1 1 1] Set Info
      (Math|Integer|IncrementInt (Variables|Default|GetStepCount)
        (:%20%20
          (Variables|Default|SetInfo (Utilities|Text|ToText(String) (Utilities|String|Append "I:" (Utilities|String|ToString(Integer) (Variables|Default|GetI)) " " "J:" (Utilities|String|ToString(Integer) (Variables|Default|GetJ)))))
          ;[1 1 1] If Items[J]<Items[J-1]
          (if (< (Variables|/Game/Blueprint/BP_Item.BP_Item_C|GetValue (Utilities|Array|Get(acopy) _items (Variables|Default|GetJ))) (Variables|/Game/Blueprint/BP_Item.BP_Item_C|GetValue (Utilities|Array|Get(acopy) _items (- (Variables|Default|GetJ) 1))))
            _)))
      (else
        ;[0.001582 0.1594 0.02441] 执行完一轮J。I++， J=I+1
        (bind _result (Math|Integer|IncrementInt (Variables|Default|GetI))
          (:%20%20
            (Variables|Default|SetJ (+ _result 1))))))))

(fn ConstructionScript
  (|CallParentFunction))

(fn MoveX
  (params (InLastIndex :type Integer) (InTargetIndex :type Integer))
  (bind _outlocation (CallFunction|GetItemLocation InLastIndex))
  (bind _outlocation_2 (CallFunction|GetItemLocation InTargetIndex))
  (Default|Move (Utilities|Array|Get(acopy) (Variables|Default|GetItems) InLastIndex) _outlocation _outlocation_2 0.0))

(fn MoveY
  (params (InLastIndex :type Integer) (InTargetIndex :type Integer))
  (bind _width (Variables|Default|GetWidth))
  (bind _returnvalue (* _width 2.0))
  (bind _returnvalue_2 (Math|Vector|MakeVector _returnvalue 0.0 0.0))
  (bind _outlocation (CallFunction|GetItemLocation InLastIndex))
  (bind _outlocation_2 (CallFunction|GetItemLocation InTargetIndex))
  (Default|Move (Utilities|Array|Get(acopy) (Variables|Default|GetItems) InLastIndex) (- _outlocation _returnvalue_2) (- _outlocation_2 _returnvalue_2) 0.0))