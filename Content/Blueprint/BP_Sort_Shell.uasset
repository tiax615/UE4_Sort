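; BP_Sort_Shell is a child Blueprint that sets up Shell sort state on top of a parent sort class.
; Init calls the parent with amount, length and sort time, then sets the gap to half the item count, starts both indices there and clears the temp reference.
; MoveX and MoveY are empty and the event graph has no active logic, so this file contains no sorting steps.
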(event EventBeginPlay
  (|CallParentFunction) ; This node is disabled and will not be called.\nDrag off pins to build functionality.
)

(event Collision|EventActorBeginOverlap
  (params (OtherActor :type Actor%20Object%20Reference)))

(event EventTick
  (params (DeltaSeconds :type Float%20%28single-precision%29)))

(fn ConstructionScript
  (|CallParentFunction))

(fn MoveX)

(fn MoveY)

(fn Init
  (params (InAmount :type Integer) (InLength :type Float%20%28single-precision%29) (InSortTime :type Float%20%28single-precision%29))
  (|CallParentFunction InAmount InLength InSortTime)
  (bind _output_get (Variables|Default|SetGap (/ (Utilities|Array|Length (Variables|Default|GetItems)) 2)))
  (bind _output_get_2 (Variables|Default|SetI _output_get))
  (Variables|Default|SetJ _output_get_2)
  (Variables|Default|SetTemp 0))