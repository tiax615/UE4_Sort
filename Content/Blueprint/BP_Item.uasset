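; BP_Item is a cube actor that represents an integer value as a bar with a numeric text label.
; SetSize, run from the construction script, derives height from the value, scales and lifts the cube, and updates the label text and scale.
; BeginPlay creates a dynamic material instance so SetColor can tint the cube.
; The Move event uses a timeline to lerp the actor to a target location.
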(event Custom|Move
  (params (MTargetLocation :type Vector))
  (Variables|Default|SetTargetLocation MTargetLocation)
  (Variables|Default|SetLastLocation (Transformation|GetActorLocation))
  (bind _coeff (Timeline|Timeline_Move Play)
    (:Update
      (Transformation|SetActorLocation (Math|Vector|Lerp(Vector) (Variables|Default|GetLastLocation) (Variables|Default|GetTargetLocation) _coeff) false false))))

(event EventBeginPlay
  (bind _returnvalue (Rendering|Material|CreateDynamicMaterialInstance (Variables|Default|GetCube) 0 "/Game/Material/MI_Color.MI_Color" "None" :!class /Script/Engine.PrimitiveComponent))
  (Variables|Default|SetMaterial _returnvalue))

(fn ConstructionScript
  (CallFunction|SetSize (Variables|Default|GetWidth) (Variables|Default|GetValue)))

(fn SetSize
  (params (MyWidth :type Float%20%28single-precision%29) (MyValue :type Integer))
  ;[1 1 1] Set Width/Height/Value
  (Variables|Default|SetWidth MyWidth)
  (bind _output_get (Variables|Default|SetValue MyValue))
  (Variables|Default|SetHeight (* _output_get (Variables|Default|GetHeightCoeff)))
  (Transformation|SetRelativeScale3D (Variables|Default|GetCube) (Math|Vector|MakeVector (/ (Variables|Default|GetWidth) 1e+02) (/ (Variables|Default|GetWidth) 1e+02) (/ (Variables|Default|GetHeight) 1e+02)))
  (Rendering|Components|TextRender|SetText (Variables|Default|GetTextRender) (Utilities|Text|ToText(Integer) (Variables|Default|GetValue) false false))
  (Transformation|SetRelativeLocation (Variables|Default|GetCube) (Math|Vector|MakeVector 0.0 0.0 (/ (Variables|Default|GetHeight) 2.0)) false false)
  (Transformation|SetRelativeScale3D (Variables|Default|GetTextRender) (Math|Conversions|ToVector(Float) (/ (Variables|Default|GetWidth) 2e+01))))

(fn SetColor
  (params (MyColor :type Linear%20Color%20Structure))
  (Rendering|Material|SetVectorParameterValue (Variables|Default|GetMaterial) "Color" MyColor :!class /Script/Engine.MaterialInstanceDynamic))